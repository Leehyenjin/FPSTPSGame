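; Actor component that simulates its owning bullet's flight with gravity and quadratic air drag, launched along the owner's forward vector.
; Each tick it line-traces to the next position, moving the owner and updating velocity when nothing is hit.
; Hits destroy the owner, damaging "Enemy"-tagged actors or leaving bullet-hole decals elsewhere.
; Debug lines draw the path colored by remaining speed; the lifetime-based destroy is disconnected, so missed bullets never expire here.
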(event `self.ReceiveBeginPlay`
  (bind _returnvalue (`self.GetOwner`))
  (set `self.BulletVelocity` (* (`Actor.GetActorForwardVector` _returnvalue) (`self.BulletSpeed`)))
  (set `self.StartLocation` (`Actor.K2_GetActorLocation` _returnvalue))
  (set `self.IsBulletInitialized` true))

(event `self.ReceiveTick`
  (params (DeltaSeconds :type "Float (single-precision)"))
  (bind _nextlocation (`self.NextLocation`))
  (if (`self.IsBulletInitialized`)
    (set `self.DeltaTime` DeltaSeconds)
    (set `self.StartLocation` (`Actor.K2_GetActorLocation` (`self.GetOwner`)))
    (set `self.NextLocation` (+ (`self.StartLocation`) (* (`self.BulletVelocity`) (`self.DeltaTime`))))
    (bind (_outhit _returnvalue) (`KismetSystemLibrary.LineTraceSingle` (`self.StartLocation`) (`self.NextLocation`) "TraceTypeQuery1" false (`|MakeArray` (`self.ActorToIgnore`)) "None" true (struct :`R` 1.0 :`A` 1.0) (struct :`G` 1.0 :`A` 1.0) 10.0))
    (bind (_bblockinghit _binitialoverlap _time _distance _location _impactpoint _normal _impactnormal _physmat _hitactor) (`GameplayStatics.BreakHitResult` _outhit))
    (`KismetSystemLibrary.DrawDebugLine` (`self.StartLocation`) (select `bool` _returnvalue :`false` _nextlocation :`true` _impactpoint) (`self.ChangeTraceColor`) 60.0)
    (if _returnvalue
      (if (`Actor.ActorHasTag` _hitactor "Enemy")
        (`GameplayStatics.ApplyDamage` _hitactor 10.0)
        (`Actor.K2_DestroyActor` (`self.GetOwner`))
        (else
          (`self.CreateBulletHole` _outhit)
          (`Actor.K2_DestroyActor` (`self.GetOwner`))))
      (else
        (`Actor.K2_SetActorLocation` (`self.GetOwner`) _nextlocation false false)
        (set `self.BulletVelocity` (`self.CalculateGravityAndDecelaration` (`self.BulletVelocity`)))))))

(fn `CalculateGravityAndDecelaration`
  (params (Velocity :type "Vector Structure"))
  (returns (ReturnValue :type "Vector Structure"))
  (return (+ Velocity (* (* (* (/ (`self.DragForce` (`self.AirDensity`) (/ (`KismetMathLibrary.VSize` Velocity) 100.0) (`self.CrossSection`) (`self.DragCoefficiency`)) (`self.BulletMass`)) 100.0) (`KismetMathLibrary.Normal` (`local.Velocity`))) (`self.DeltaTime`)) (`KismetMathLibrary.MakeVector` 0.0 0.0 (* (* (`self.Gravity`) -100.0) (`self.DeltaTime`))))))

(fn `ChangeTraceColor`
  (returns (ReturnValue :type "LinearColor Structure"))
  (bind _returnvalue (/ (`KismetMathLibrary.VSize` (`self.BulletVelocity`)) (`self.BulletSpeed`)))
  (if (> _returnvalue 0.75)
    (return (`KismetMathLibrary.LinearColorLerp` (struct :`R` 1.0 :`G` 0.571125 :`B` 0.023153 :`A` 1.0) (struct :`R` 1.0 :`G` 0.047707 :`A` 1.0) (`KismetMathLibrary.NormalizeToRange` _returnvalue 0.0 1.0)))
    (elif (> _returnvalue 0.5)
      (return (`KismetMathLibrary.LinearColorLerp` (struct :`R` 1.0 :`G` 0.812529 :`A` 1.0) (struct :`R` 1.0 :`G` 0.571125 :`B` 0.023153 :`A` 1.0) (`KismetMathLibrary.NormalizeToRange` _returnvalue 0.0 1.0)))
      (elif (> _returnvalue 0.25)
        (return (`KismetMathLibrary.LinearColorLerp` (struct :`R` 0.011733 :`G` 1.0 :`B` 0.0532 :`A` 1.0) (struct :`R` 1.0 :`G` 0.814847 :`A` 1.0) (`KismetMathLibrary.NormalizeToRange` _returnvalue 0.0 1.0)))
        (else
          (return (`KismetMathLibrary.LinearColorLerp` (struct :`R` 0.008226 :`G` 0.107856 :`B` 1.0 :`A` 1.0) (struct :`R` 0.011612 :`G` 1.0 :`B` 0.052861 :`A` 1.0) (`KismetMathLibrary.NormalizeToRange` _returnvalue 0.0 1.0))))))))

(fn `CreateBulletHole`
  (params (HitResult :type "HitResult Structure"))
  (bind (_bblockinghit _binitialoverlap _time _distance _location _impactpoint _normal _impactnormal) (`GameplayStatics.BreakHitResult` HitResult))
  (bind _returnvalue (`GameplayStatics.SpawnDecalAtLocation` "/Game/CustomContents/Weapons/Bullet/Mrtl_BulletHole.Mrtl_BulletHole" (1.0 10.0 10.0) _location (`KismetMathLibrary.MakeRotFromX` _impactnormal)))
  (`DecalComponent.SetFadeScreenSize` _returnvalue 0.01))

(fn `DragForce`
  (params (AirDensity :type "Float (double-precision)") (BulletSpeed :type "Float (double-precision)") (CrossSection :type "Float (double-precision)") (DragCoefficiency :type "Float (double-precision)"))
  (returns (ReturnValue :type "Float (double-precision)"))
  (return (* (/ (* (* (* AirDensity (`KismetMathLibrary.Square` BulletSpeed)) CrossSection) DragCoefficiency) 2.0) -1.0)))