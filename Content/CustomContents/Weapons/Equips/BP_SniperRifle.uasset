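; BP_SniperRifle is a sniper rifle weapon Blueprint with a live scope view rendered onto its lens.
; Its construction script creates a render target per instance and assigns it to a SceneCaptureComponent2D.
; A dynamic material on the Lens mesh takes that target as a texture parameter, giving a picture-in-picture scope.
; The event graph holds only disabled default events, so any other behavior comes from the parent class.
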(fn `UserConstructionScript`
  (`parent.UserConstructionScript`)
  (bind _returnvalue (`KismetRenderingLibrary.CreateRenderTarget2D` 1000 1000))
  (bind _output_get (set `SceneCaptureComponent2D.TextureTarget` _returnvalue (`self.SceneCaptureComponent2D`)))
  (bind _returnvalue_2 (`PrimitiveComponent.CreateDynamicMaterialInstance` (`self.Lens`) 0 (`PrimitiveComponent.GetMaterial` (`self.Lens`) 0) "None"))
  (`MaterialInstanceDynamic.SetTextureParameterValue` _returnvalue_2 "Target" _output_get)
  (`PrimitiveComponent.SetMaterial` (`self.Lens`) 0 _returnvalue_2))