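; BP_Rocket is a rocket projectile actor that explodes on contact or when its lifetime runs out.
; BeginPlay waits for the Time delay, while the ContactSensor component triggers the same blast on any overlap, without filtering the other actor.
; Both paths spawn the rocket launcher explosion particle and sound at the actor's location, then destroy it.
; These graphs apply no damage.
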(event `self.ReceiveBeginPlay`
  (`KismetSystemLibrary.Delay` (`self.Time`))
  (`GameplayStatics.SpawnEmitterAtLocation` "/Game/MilitaryWeapDark/FX/P_RocketLauncher_Explosion_01.P_RocketLauncher_Explosion_01" (`self.K2_GetActorLocation`))
  (`GameplayStatics.PlaySoundAtLocation` "/Game/CustomContents/Weapons/Rocket/SC_RandomExplosionSound.SC_RandomExplosionSound" (`self.K2_GetActorLocation`) (struct) 1.0 1.0 0.0 null null null null)
  (`self.K2_DestroyActor`))

(event `self.ContactSensor.OnComponentBeginOverlap`
  (params (OverlappedComponent :type "PrimitiveComponent Object Reference") (OtherActor :type "Actor Object Reference") (OtherComp :type "PrimitiveComponent Object Reference") (OtherBodyIndex :type Integer) (bFromSweep :type Boolean) (SweepResult :type "HitResult Structure (by ref)"))
  ;[1 1 1] 이펙트효과 나타났다 사라짐
  (`GameplayStatics.SpawnEmitterAtLocation` "/Game/MilitaryWeapDark/FX/P_RocketLauncher_Explosion_01.P_RocketLauncher_Explosion_01" (`self.K2_GetActorLocation`))
  (`GameplayStatics.PlaySoundAtLocation` "/Game/CustomContents/Weapons/Rocket/SC_RandomExplosionSound.SC_RandomExplosionSound" (`self.K2_GetActorLocation`) (struct) 1.0 1.0 0.0 null null null null)
  (`self.K2_DestroyActor`))

(fn `UserConstructionScript`)