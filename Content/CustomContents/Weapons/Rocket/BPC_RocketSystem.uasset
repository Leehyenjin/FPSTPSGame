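; BPC_RocketSystem is a component that propels its owning BP_Rocket with physics forces.
; BeginPlay casts the owner to BP_Rocket and caches it.
; Every Tick applies two forces to the rocket's mesh: Thrust along the owner's forward vector and UpThrust along its up vector.
; The forces are mass-dependent, since AccelChange is off.
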(event `self.ReceiveBeginPlay`
  (bind _asbp_rocket (cast `/Game/CustomContents/Weapons/Rocket/BP_Rocket` (`self.GetOwner`)))
  (set `self.Rocket` _asbp_rocket))

(event `self.ReceiveTick`
  (params (DeltaSeconds :type "Float (single-precision)"))
  (bind _returnvalue (`self.GetOwner`))
  ;[1 1 1] 로켓이 앞으로 매 틱마다 3000씩 움직인다 위로는 300씩
  (`PrimitiveComponent.AddForce` (`/Game/CustomContents/Weapons/Rocket/BP_Rocket.RocketMesh` (`self.Rocket`)) (* (`Actor.GetActorForwardVector` _returnvalue) (`self.Thrust`)) "None" false)
  (`PrimitiveComponent.AddForce` (`/Game/CustomContents/Weapons/Rocket/BP_Rocket.RocketMesh` (`self.Rocket`)) (* (`Actor.GetActorUpVector` _returnvalue) (`self.UpThrust`)) "None" false))